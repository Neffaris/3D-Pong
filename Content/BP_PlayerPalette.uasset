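; BP_PlayerPalette is a player-named actor with a CharacterMovement component, kept within a fixed range along world X.
; Each Tick checks its location and snaps X back to the nearer limit when it leaves that range, preserving Y and Z.
; Tick also prints X velocity as a fraction of max movement speed for on-screen debugging.
; The graphs contain no input handling, and the construction script is empty.
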(event EventTick
  (params (DeltaSeconds :type Float%20%28single-precision%29))
  (bind _returnvalue (Transformation|GetActorLocation))
  (if (> (.x _returnvalue) -2.6e+02)
    (Transformation|SetActorLocation (Math|Vector|MakeVector -2.6e+02 (.y _returnvalue) (.z _returnvalue)) false false)
    (elif (< (.x _returnvalue) -8.4e+02)
      (Transformation|SetActorLocation (Math|Vector|MakeVector -8.4e+02 (.y _returnvalue) (.z _returnvalue)) false false)))
  (Development|PrintString (Utilities|String|ToString(Float) (/ (.x (Transformation|GetVelocity)) (Class|MovementComponent|GetMaxSpeed (Variables|Character|GetCharacterMovement)))) true true "(R=0.000000,G=1.000000,B=0.043140,A=1.000000)" 0.0))

(fn ConstructionScript)